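; Game state that tracks how many floating mushrooms and chests the player has collected and how many remain in the level.
; On BeginPlay it counts all mushroom and chest actors as totals, then computes the remaining amounts.
; Separate events increment each collected count or recalculate what is left, updating the remainder only while it stays non-negative.
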(event `self.ReceiveBeginPlay`
  (`self.setTotalObjectsNumber`)
  (`self.setChestsLeft`)
  (`self.setMushroomsLeft`))

(event `setMushroomsCollected`
  (set `self.mushroomCollected` (+ (`self.mushroomCollected`) 1)))

(event `setChestsCollected`
  (set `self.chestsCollected` (+ (`self.chestsCollected`) 1)))

(event `setMushroomsLeft`
  (bind _returnvalue (- (`self.totalMushrooms`) (`self.mushroomCollected`)))
  (if (>= _returnvalue 0)
    (set `self.mushroomsLeft` _returnvalue)))

(event `setChestsLeft`
  (bind _returnvalue (- (`self.totalChests`) (`self.chestsCollected`)))
  (if (>= _returnvalue 0)
    (set `self.chestsLeft` _returnvalue)))

(fn `setTotalObjectsNumber`
  (`|ExecutionSequence`
    (:`then_0`
      (bind _outactors (`GameplayStatics.GetAllActorsOfClass` "/Game/Blueprints/Mushroom/BP_floatingMushroom.BP_floatingMushroom_C"))
      (set `self.totalMushrooms` (`KismetArrayLibrary.Array_Length` _outactors)))
    (:`then_1`
      (bind _outactors_2 (`GameplayStatics.GetAllActorsOfClass` "/Game/Blueprints/Chest/chestFinal_Blueprint.chestFinal_Blueprint_C"))
      (set `self.totalChests` (`KismetArrayLibrary.Array_Length` _outactors_2)))))

(fn `UserConstructionScript`)