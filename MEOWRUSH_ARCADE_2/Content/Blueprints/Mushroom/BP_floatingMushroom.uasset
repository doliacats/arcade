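; BP_floatingMushroom is a collectible mushroom that BP_Cat picks up by overlapping its Box.
; A timeline started on BeginPlay drives the mesh's height offset, lerping its relative location from the actor's world start location, while Tick spins it around yaw.
; On pickup it updates the collected and remaining mushroom counts in gs_gamestate, spawns a shockwave effect and destroys itself.
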(event `self.ReceiveBeginPlay`
  (bind _startlocation (`self.startLocation`))
  (set `self.startLocation` (`self.K2_GetActorLocation`))
  (bind (_direction _tl_track) (`Timeline|tl_floating`)
    (:`Update`
      (`SceneComponent.K2_SetRelativeLocation` (`self.Mushroom`) (`KismetMathLibrary.VLerp` _startlocation (+ _startlocation (0.0 0.0 50.0)) _tl_track) false false))))

(event `self.ReceiveTick`
  (params (DeltaSeconds :type "Float (single-precision)"))
  (`SceneComponent.K2_AddLocalRotation` (`self.Mushroom`) (`KismetMathLibrary.MakeRotator` 0.0 0.0 (* DeltaSeconds (`self.rotationSpeed`))) false false))

(event `self.Box.OnComponentBeginOverlap`
  (params (OverlappedComponent :type "PrimitiveComponent Object Reference") (OtherActor :type "Actor Object Reference") (OtherComp :type "PrimitiveComponent Object Reference") (OtherBodyIndex :type Integer) (bFromSweep :type Boolean) (SweepResult :type "HitResult Structure (by ref)"))
  (cast `/Game/Blueprints/Cat/BP_Cat` OtherActor)
  (bind _asgs_gamestate (cast `/Game/Blueprints/gs_gamestate` (`GameplayStatics.GetGameState`)))
  (`/Game/Blueprints/gs_gamestate.setMushroomsCollected` _asgs_gamestate)
  (`/Game/Blueprints/gs_gamestate.setMushroomsLeft` _asgs_gamestate)
  (`GameplayStatics.SpawnEmitterAtLocation` "/Game/Blueprints/Mushroom/fx_shockwave.fx_shockwave" (`self.K2_GetActorLocation`))
  (`self.K2_DestroyActor`))

(fn `UserConstructionScript`)